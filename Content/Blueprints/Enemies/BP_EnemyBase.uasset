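; Base enemy that sweeps in, patrols back and forth, and damages the player on contact.
; BeginPlay increments the game mode's live count, randomizes speed and direction, then runs a timeline slide along Y before enabling Tick-driven Z movement.
; Hits on non-enemies reverse direction and damage players.
; AnyDamage sets health to clamped damage minus health (reversed subtraction), decrementing the count and destroying the actor at zero.
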(event `self.ReceiveBeginPlay`
  (bind _spawnlocation (`self.SpawnLocation`))
  ;[1 1 1] Random Movement Direction
  (bind _asmy_game_mode (cast `/Game/Blueprints/MyGameMode` (`GameplayStatics.GetGameMode`)))
  (bind _output_get (set `self.BpGameMode` _asmy_game_mode))
  (set `/Game/Blueprints/MyGameMode.LiveEnemies` (+ (`/Game/Blueprints/MyGameMode.LiveEnemies` _output_get) 1) _output_get)
  (set `self.bMoveDirection` (`KismetMathLibrary.RandomBool`))
  (set `self.MoveSpeed` (`KismetMathLibrary.RandomFloatInRange` 500.0 1000.0))
  (set `self.Sweepin` (`KismetMathLibrary.RandomFloatInRange` 1200.0 -1200.0))
  ;[1 1 1] Spawn Animation
  (set `self.SpawnLocation` (`self.K2_GetActorLocation`))
  (bind (_direction _speed) (`Timeline|SpawnAnimation`)
    (:`Update`
      (`self.K2_SetActorLocation` (`KismetMathLibrary.VLerp` _spawnlocation (- _spawnlocation (`KismetMathLibrary.MakeVector` 0.0 (`self.Sweepin`))) _speed) true))
    (:`Finished`
      (set `self.bMoveEnabled` true))))

(event `self.ReceiveTick`
  (params (DeltaSeconds :type "Float (single-precision)"))
  ;[1 1 1] Movement
  (if (`self.bMoveEnabled`)
    (`self.K2_SetActorLocation` (+ (`self.K2_GetActorLocation`) (* (`KismetMathLibrary.GreaterGreater_VectorRotator` (`KismetMathLibrary.MakeVector` 0.0 0.0 (* (`self.MoveSpeed`) (`KismetMathLibrary.SelectFloat` 1.0 -1.0 (`self.bMoveDirection`))))) DeltaSeconds)) true)))

(event `self.ReceiveHit`
  (params (MyComp :type "PrimitiveComponent Object Reference") (Other :type "Actor Object Reference") (OtherComp :type "PrimitiveComponent Object Reference") (bSelfMoved :type Boolean) (HitLocation :type "Vector Structure") (HitNormal :type "Vector Structure") (NormalImpulse :type "Vector Structure") (Hit :type "HitResult Structure (by ref)"))
  ;[1 1 1] Death
  (cast `/Game/Blueprints/Enemies/BP_EnemyBase` Other
    (:`CastFailed`
      (set `self.bMoveDirection` (not (`self.bMoveDirection`)))
      (bind _asbp_player (cast `/Game/Blueprints/BP_Player` Other))
      (`GameplayStatics.ApplyDamage` _asbp_player 50.0))))

(event `self.ReceiveAnyDamage`
  (params (Damage :type "Float (single-precision)") (DamageType :type "DamageType Object Reference") (InstigatedBy :type "Controller Object Reference") (DamageCauser :type "Actor Object Reference"))
  (bind _bpgamemode (`self.BpGameMode`))
  ;[1 1 1] Death
  (set `self.Health` (`KismetMathLibrary.FClamp` (- Damage (`self.Health`)) 0.0 (`self.MaxHealth`)))
  (if (<= (`self.Health`) 0.0)
    (set `/Game/Blueprints/MyGameMode.LiveEnemies` (- (`/Game/Blueprints/MyGameMode.LiveEnemies` _bpgamemode) 1) _bpgamemode)
    (`self.K2_DestroyActor`)))

(fn `UserConstructionScript`
  (set `self.Health` (`self.MaxHealth`)))