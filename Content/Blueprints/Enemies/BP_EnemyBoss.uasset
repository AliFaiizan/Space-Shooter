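; Boss enemy Blueprint that repeatedly fires a pair of projectiles, extending the behavior of its parent class.
; Tick runs the parent logic, then uses a Delay of FireRate as a repeating fire timer, since retriggers are ignored while it is pending.
; Each cycle spawns BP_EnemyProjectile at the Top and Bottom component transforms, with fixed damage and velocity along negative Y.
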(event `self.ReceiveTick`
  (params (DeltaSeconds :type "Float (single-precision)"))
  (`parent.ReceiveTick` DeltaSeconds)
  (`KismetSystemLibrary.Delay` (`self.FireRate`))
  (`|SpawnActorFromClass` "/Game/Blueprints/BP_EnemyProjectile.BP_EnemyProjectile_C" (`SceneComponent.K2_GetComponentToWorld` (`self.Top`)) "Undefined" "OverrideRootScale" null 5.0 (0.0 -2200.0 0.0) (1.0 1.0 1.0) null)
  (`|SpawnActorFromClass` "/Game/Blueprints/BP_EnemyProjectile.BP_EnemyProjectile_C" (`SceneComponent.K2_GetComponentToWorld` (`self.bottom`)) "Undefined" "OverrideRootScale" null 5.0 (0.0 -2200.0 0.0) (1.0 1.0 1.0) null))

(fn `UserConstructionScript`
  (`parent.UserConstructionScript`))