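; BP_Projectile_Rockets is a rocket projectile with homing logic that currently targets BP_Player, noted as a placeholder for an enemy class.
; The HommingBox overlap stores the first player it detects in TempVar while no valid target is held.
; Tick lerps ProjectileMovement velocity toward that target at ChangedSpeed, but the lerp alpha is zero, so the steering has no effect as written.
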(event `self.ReceiveTick`
  (params (DeltaSeconds :type "Float (single-precision)"))
  (`parent.ReceiveTick` DeltaSeconds)
  (`/Engine/EditorBlueprintResources/StandardMacros.IsValid` (`self.TempVar`)
    (:`Is Valid`
      (set `MovementComponent.Velocity` (`KismetMathLibrary.VLerp` (`MovementComponent.Velocity` (`self.ProjectileMovement`)) (* (`KismetMathLibrary.Normal` (- (`self.K2_GetActorLocation` (`self.TempVar`)) (`self.K2_GetActorLocation`))) (`self.ChangedSpeed`))) (`self.ProjectileMovement`)))))

(event `self.homming box.OnComponentBeginOverlap`
  (params (OverlappedComponent :type "PrimitiveComponent Object Reference") (OtherActor :type "Actor Object Reference") (OtherComp :type "PrimitiveComponent Object Reference") (OtherBodyIndex :type Integer) (bFromSweep :type Boolean) (SweepResult :type "HitResult Structure (by ref)"))
  ;[1 0.07657 0] Replace With Enemy
  (bind _asbp_player (cast `/Game/Blueprints/BP_Player` OtherActor))
  (`/Engine/EditorBlueprintResources/StandardMacros.IsValid` (`self.TempVar`)
    (:`Is Not Valid`
      (set `self.TempVar` _asbp_player))))

(fn `UserConstructionScript`
  (`parent.UserConstructionScript`))