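; Enemy spawner actor that runs three sequential waves of enemies, coordinated through MyGameMode.
; A looping timer calls CheckWave, which starts the next wave when the game mode reports no live enemies.
; BeginWave resets the spawn counter and publishes the wave size to the game mode.
; SpawnWave immediately spawns random classes from that wave's list at fixed X/Y and random Z within game mode bounds.
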(event `self.ReceiveBeginPlay`
  (bind _asmy_game_mode (cast `/Game/Blueprints/MyGameMode` (`GameplayStatics.GetGameMode`)))
  (set `self.bpGamemode` _asmy_game_mode)
  (bind _returnvalue (`KismetSystemLibrary.K2_SetTimer` null "CheckWave" 0.5 true))
  (set `self.waveTimer` _returnvalue))

(event `CheckWave`
  (bind _output (`|GetArrayItem` (`self.EnemyCount`) (`self.WaveIndex`)))
  (if (and (== (`/Game/Blueprints/MyGameMode.LiveEnemies` (`self.bpGamemode`)) 0) (`self.bWaveReady`))
    (switch `int` (`self.WaveIndex`)
      (:`0`
        (`self.Begin Wave` _output)
        (`self.Spawn Wave` _output (`self.EnemyWave1`)))
      (:`1`
        (`self.Begin Wave` _output)
        (`self.Spawn Wave` _output (`self.EnemyWave2`)))
      (:`2`
        (`self.Begin Wave` _output)
        (`self.Spawn Wave` _output (`self.EnemyWave3`))))
    (set `self.WaveIndex` (+ (`self.WaveIndex`) 1))))

(fn `Begin Wave`
  (params (`Wave Total` :type Integer))
  (bind _bpgamemode (`self.bpGamemode`))
  (set `self.bWaveReady` true)
  (set `self.waveActive` 0)
  (set `/Game/Blueprints/MyGameMode.MaxWave` `Wave Total` _bpgamemode)
  (set `/Game/Blueprints/MyGameMode.ActiveWave` `Wave Total` _bpgamemode))

(fn `Spawn Wave`
  (params (WaveTotal :type Integer) (WaveEnemies :type "Array of /Game/Blueprints/Enemies/BP_EnemyBase Class Reference"))
  (bind _bpgamemode (`self.bpGamemode`))
  (bind (_bpspawnminvalue_x _bpspawnminvalue_y _bpspawnminvalue_z) (`KismetMathLibrary.BreakVector` (`/Game/Blueprints/MyGameMode.bpSpawnMinValue` _bpgamemode)))
  (bind (_bpspawnmaxvalue_x _bpspawnmaxvalue_y _bpspawnmaxvalue_z) (`KismetMathLibrary.BreakVector` (`/Game/Blueprints/MyGameMode.bpSpawnMaxValue` _bpgamemode)))
  (for _ (range (+ (+ WaveTotal 1) 1))
    (if (> WaveTotal (`self.waveActive`))
      (if (`self.bWaveReady`)
        (`|SpawnActorFromClass` (`|GetArrayItem` WaveEnemies (`KismetMathLibrary.RandomInteger` (`KismetArrayLibrary.Array_Length` WaveEnemies))) (`KismetMathLibrary.MakeTransform` (`KismetMathLibrary.MakeVector` _bpspawnminvalue_x _bpspawnminvalue_y (`KismetMathLibrary.RandomFloatInRange` _bpspawnminvalue_z _bpspawnmaxvalue_z))) "AlwaysSpawn" "OverrideRootScale" null null)
        (set `self.waveActive` (+ (`self.waveActive`) 1)))
      (else
        (set `self.bWaveReady` true)))))

(fn `UserConstructionScript`)