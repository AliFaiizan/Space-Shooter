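; Player pawn for a shooter played on the Y-Z plane, with a spinning fly-in on spawn that enables movement when finished.
; Tick eases input into vertical and horizontal speeds, moves the actor and tilts the mesh to match.
; Input-opened gates and countdown timers pace primary fire (randomized height, or multi-shot with power-up) and rocket volleys when owned.
; Damage reduces clamped health and flags PlayerDead on MyGameMode at zero.
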(event `self.ReceiveBeginPlay`
  (bind _spawn_location (`self.Spawn Location`))
  (set `self.Health` (`self.max Health`))
  (set `self.Pitch` (.pitch (`SceneComponent.RelativeRotation` (`self.PlayerMesh`))))
  (set `self.Spawn Location` (`self.K2_GetActorLocation`))
  (set `self.Spawn Rotation` (`SceneComponent.K2_GetComponentRotation` (`self.PlayerMesh`)))
  (bind (_direction _spawntime) (`Timeline|SpawnAnimation`)
    (:`Update`
      (`self.K2_SetActorLocation` (`KismetMathLibrary.VLerp` _spawn_location (+ _spawn_location (0.0 1000.0 0.0)) _spawntime) true)
      (`SceneComponent.K2_SetRelativeRotation` (`self.PlayerMesh`) (`KismetMathLibrary.RLerp` (`self.Spawn Rotation`) (`KismetMathLibrary.MakeRotator` 0.0 (+ (`self.Pitch`) 720.0)) _spawntime) false false))
    (:`Finished`
      (set `self.bMovementEnabled` true))))

(event `self.ReceiveTick`
  (params (DeltaSeconds :type "Float (single-precision)"))
  ;[1 1 1] Movement
  (set `self.Delta Seconds` DeltaSeconds)
  (if (`self.bMovementEnabled`)
    (`self.Fire Rate Controll`)
    (`|ExecutionSequence`
      (:`then_0`
        (bind _current_speed (`self.Get Direction` (`self.Vertical Speed`) (`self.GetInputAxisValue`)))
        (set `self.Vertical Speed` _current_speed))
      (:`then_1`
        (bind _current_speed_2 (`self.Get Direction` (`self.Horizontal Speed`) (`self.GetInputAxisValue`)))
        (set `self.Horizontal Speed` _current_speed_2))
      (:`then_2`
        (`self.K2_SetActorLocation` (+ (`self.K2_GetActorLocation`) (`KismetMathLibrary.MakeVector` 0.0 0.0 (`self.Vertical Speed`))))
        (`self.K2_SetActorLocation` (+ (`self.K2_GetActorLocation`) (`KismetMathLibrary.MakeVector` 0.0 (`self.Horizontal Speed`))))
        (if (>= (`self.Health`) 0.0)
          (`SceneComponent.K2_SetRelativeRotation` (`self.PlayerMesh`) (`KismetMathLibrary.RInterpTo` (`self.K2_GetActorRotation`) (`KismetMathLibrary.MakeRotator` (* (`self.Horizontal Speed`) -1.0) (* (`self.Vertical Speed`) 4.0)) (`self.Delta Seconds`) 20.0) false false))))))

(event `InputAction|Primary Fire`
  (params (Key :type "Key Structure"))
  (bind _spawnloc (`self.SpawnLOC`))
  ;[1 1 1] Fire RAte Controo
  (:`Pressed`
    (goto _label :!via `Open`))
  (:`Released`
    (goto _label :!via `Close`)))

(event `Fire Rate Controll`
  (bind _spawnloc (`self.SpawnLOC`))
  ;[1 1 1] Fire RAte Controo
  (`|ExecutionSequence`
    (:`then_0`
      (bind _output_get (set `self.Primary Fire Rate` (- (`self.Primary Fire Rate`) (`self.Delta Seconds`))))
      (if (<= _output_get 0.0)
        (`/Engine/EditorBlueprintResources/StandardMacros.Gate` true :!label _label
          (:`Exit`
            (set `self.Primary Fire Rate` (`self.Primary Fire Rate Base`))
            (if (`self.bHasPower`)
              (`self.PowerUp Fire` _spawnloc (`self.PowerUp FireRate`))
              (else
                (`self.PrimaryFire` _spawnloc)))))))
    (:`then_1`
      (bind _output_get_2 (set `self.Secondary Fire Rate` (- (`self.Secondary Fire Rate`) (`self.Delta Seconds`))))
      (if (<= _output_get_2 0.0)
        (`/Engine/EditorBlueprintResources/StandardMacros.Gate` true :!label _label_2
          (:`Exit`
            (set `self.Secondary Fire Rate` (`self.Secondary Fire Rate Base`))
            (if (`self.bHasRockets`)
              (`self.Secondary Fire` _spawnloc (`self.SecondaryShot Fire Rate`)))))))))

(event `InputAction|Secondary Fire`
  (params (Key :type "Key Structure"))
  ;[1 1 1] Fire RAte Controo
  (:`Pressed`
    (goto _label_2 :!via `Open`))
  (:`Released`
    (goto _label_2 :!via `Close`)))

(event `self.ReceiveAnyDamage`
  (params (Damage :type "Float (single-precision)") (DamageType :type "DamageType Object Reference") (InstigatedBy :type "Controller Object Reference") (DamageCauser :type "Actor Object Reference"))
  ;[1 1 1] Event Damagae
  (set `self.Health` (`KismetMathLibrary.FClamp` (- (`self.Health`) Damage) 0.0 (`self.max Health`)))
  (if (<= (`self.Health`) 0.0)
    (bind _asmy_game_mode (cast `/Game/Blueprints/MyGameMode` (`GameplayStatics.GetGameMode`)))
    (set `/Game/Blueprints/MyGameMode.PlayerDead` true _asmy_game_mode)))

(fn `Get Direction`
  (params (Speed :type "Float (double-precision)") (GetDirection :type "Float (double-precision)"))
  (returns (`Current Speed` :type "Float (double-precision)"))
  (bind _delta_seconds (`self.Delta Seconds`))
  (bind _output_get (set `self.CurrentSpeed` (`KismetMathLibrary.FInterpTo` Speed (* (* GetDirection (`self.MoveSpeed`)) _delta_seconds) _delta_seconds 4.0)))
  (return _output_get))

(fn `PowerUp Fire`
  (params (SpawnLocation :type "SceneComponent Object Reference") (`Shots Fired` :type Integer))
  (locals (Offset :type Integer))
  (bind _returnvalue (`SceneComponent.K2_GetComponentToWorld` SpawnLocation))
  (bind _returnvalue_2 (+ (.z (.location _returnvalue)) (* (`KismetMathLibrary.Conv_IntToDouble` (`local.Offset`)) 5.0)))
  (set `local.Offset` (/ `Shots Fired` -2))
  (for _ (range (+ `Shots Fired` 1))
    (`|SpawnActorFromClass` "/Game/Blueprints/BP_Projectile_Primary.BP_Projectile_Primary_C" (`KismetMathLibrary.MakeTransform` (`KismetMathLibrary.MakeVector` (.x (.location _returnvalue)) (.y (.location _returnvalue)) _returnvalue_2) (`KismetMathLibrary.MakeRotator` _returnvalue_2)) "AlwaysSpawn" "OverrideRootScale" null null)
    (set `local.Offset` (+ (`local.Offset`) 1))))

(fn `PrimaryFire`
  (params (SceneComponent :type "SceneComponent Object Reference"))
  (bind _returnvalue (`SceneComponent.K2_GetComponentToWorld` SceneComponent))
  (`|SpawnActorFromClass` "/Game/Blueprints/BP_Projectile_Primary.BP_Projectile_Primary_C" (`KismetMathLibrary.MakeTransform` (`KismetMathLibrary.MakeVector` (.x (.location _returnvalue)) (.y (.location _returnvalue)) (+ (.z (.location _returnvalue)) (`KismetMathLibrary.RandomFloatInRange` -70.0 70.0))) (.rotation _returnvalue)) "AlwaysSpawn" "OverrideRootScale" null null))

(fn `Secondary Fire`
  (params (`Spawn Lcoation` :type "SceneComponent Object Reference") (`Shots to Fire` :type Integer))
  (locals (Offset :type Integer))
  (bind _returnvalue (`SceneComponent.K2_GetComponentToWorld` `Spawn Lcoation`))
  (set `local.Offset` (/ (+ `Shots to Fire` 1) -1))
  (for _ (range (+ `Shots to Fire` 1))
    (`|SpawnActorFromClass` "/Game/Blueprints/BP_Projectile_Rockets.BP_Projectile_Rockets_C" (`KismetMathLibrary.MakeTransform` (`KismetMathLibrary.MakeVector` (.x (.location _returnvalue)) (.y (.location _returnvalue)) (+ (.z (.location _returnvalue)) (* (`KismetMathLibrary.Conv_IntToDouble` (`local.Offset`)) 5.0)))) "AlwaysSpawn" "OverrideRootScale" null null)
    (set `local.Offset` (+ (`local.Offset`) 4))))

(fn `UserConstructionScript`)